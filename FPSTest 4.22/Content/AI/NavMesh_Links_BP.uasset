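; Nav link Blueprint that makes BasicNPC agents jump when they reach its smart link.
; On SmartLinkReached it computes a ballistic velocity from the link actor's own location, not the agent's, to the destination and launches the character with it, overriding current velocity.
; CalculateVelocity solves for a fixed JumpDuration flight time, compensating the vertical axis for a hard-coded gravity constant.
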(event EventSmartLinkReached
  (params (Agent :type Actor%20Object%20Reference) (Destination :type Vector%20%28by%20ref%29 :default "0, 0, 0"))
  (bind _asbasic_npc (Utilities|Casting|CastToBasicNPC Agent))
  (bind _finalvelocity (CallFunction|CalculateVelocity (Variables|Jump|GetJumpDuration) Destination (Transformation|GetActorLocation)))
  (Character|LaunchCharacter _asbasic_npc _finalvelocity true true))

(fn ConstructionScript)

(fn CalculateVelocity
  (params (Duration :type Float%20%28single-precision%29) (EndLocation :type Vector) (StartLocation :type Vector))
  (bind (_x _y _z) (Math|Vector|BreakVector StartLocation))
  (bind (_x_2 _y_2 _z_2) (Math|Vector|BreakVector EndLocation))
  (LocalVariables|SetInDuration Duration)
  (return (Math|Vector|MakeVector (/ (- _x_2 _x) (LocalVariables|GetInDuration)) (/ (- _y_2 _y) (LocalVariables|GetInDuration)) (/ (- _z_2 (+ _z (* (Math|Float|Square (LocalVariables|GetInDuration)) -0.5 982.0))) (LocalVariables|GetInDuration)))))