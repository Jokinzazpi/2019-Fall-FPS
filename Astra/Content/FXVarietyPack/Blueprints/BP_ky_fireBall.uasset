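; BP_ky_fireBall is a fireball projectile from FXVarietyPack that spawns a tinted shot shockwave effect on BeginPlay.
; Each tick it moves its Sphere component along the normalized MoveDir at MySpeed, without sweeping.
; Overlapping anything other than a BaseEnemy prints a debug string, spawns HitFx and destroys the actor.
; BaseEnemy overlaps are ignored, and no damage is applied here.
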(event OnComponentBeginOverlap(Sphere)
  (params (OverlappedComponent :type Primitive%20Component%20Object%20Reference) (OtherActor :type Actor%20Object%20Reference) (OtherComp :type Primitive%20Component%20Object%20Reference) (OtherBodyIndex :type Integer) (bFromSweep :type Boolean) (SweepResult :type Hit%20Result%20Structure%20%28by%20ref%29))
  ;[1 1 1] spawn collison fx
  (Utilities|Casting|CastToBaseEnemy OtherActor
    (:CastFailed
      (Development|PrintString "destroyed")
      (Effects|SpawnEmitteratLocation (Variables|Default|GethitFx) (Transformation|GetWorldLocation (Variables|Default|GetSphere)))
      ;[1 1 1] fx destroy
      (Actor|DestroyActor))))

(event EventBeginPlay
  ;[1 1 1] spawn shot shockwave
  (bind _returnvalue (Effects|SpawnEmitteratLocation "/Game/FXVarietyPack/Particles/P_ky_shotShockwave.P_ky_shotShockwave" (Transformation|GetWorldLocation (Variables|Default|GetSphere)) (Transformation|GetWorldRotation (Variables|Default|GetSphere))))
  (Effects|Components|ParticleSystem|SetVectorParameter _returnvalue "color" (Math|Conversions|ToVector(LinearColor) (Variables|Default|Getcolor))))

(event EventTick
  (params (DeltaSeconds :type Float%20%28single-precision%29))
  (bind _sphere (Variables|Default|GetSphere))
  ;[1 1 1] duration increment for control
  (Transformation|SetWorldLocation _sphere (+ (Transformation|GetWorldLocation _sphere) (* (Math|Vector|Normalize (Variables|Default|GetMoveDir)) (* (Variables|Default|GetMySpeed) (Utilities|Time|GetWorldDeltaSeconds)))) false false))

(fn ConstructionScript)