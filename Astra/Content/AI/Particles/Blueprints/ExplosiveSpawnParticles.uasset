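; ExplosiveSpawnParticles is an effect Blueprint that moves and rotates a particle component, apparently for an explosive spawn effect.
; On BeginPlay a timeline drives the FX's relative X and Z offsets, scaled by Length and Hight.
; Tick spins the Pivot in yaw at the Rotation rate for the first 0.2 seconds.
; The construction script passes Color to the FX's "color" vector parameter.
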(event EventBeginPlay
  ;[1 1 1] effect move control
  (bind (_direction _x _z) (Timeline|Timeline_0 PlayFromStart)
    (:Update
      (Transformation|SetRelativeLocation (Variables|Default|GetFX) (Math|Vector|MakeVector (* (Variables|Default|Getlength) _x) 0.0 (* (Variables|Default|Gethight) _z)) false false))))

(event EventTick
  (params (DeltaSeconds :type Float%20%28single-precision%29))
  ;[1 1 1] rotation control
  (bind _output_get (Variables|Default|Setduration (+ DeltaSeconds (Variables|Default|Getduration))))
  (if (< _output_get 0.2)
    (Transformation|AddRelativeRotation (Variables|Default|Getpivot) (Math|Rotator|MakeRotator 0.0 0.0 (* (Utilities|Time|GetWorldDeltaSeconds) (Variables|Default|Getrotation))) false false)))

(fn ConstructionScript
  ;[1 1 1] color control
  (Effects|Components|ParticleSystem|SetVectorParameter (Variables|Default|GetFX) "color" (Math|Conversions|ToVector(LinearColor) (Variables|Default|Getcolor))))