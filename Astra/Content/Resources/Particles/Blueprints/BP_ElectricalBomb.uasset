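; Electrical effect actor that repeatedly spawns BP_SpawnedArc lightning bolts around a flickering, optionally hidden glowing core.
; Arcing re-triggers itself at random delays, spawning only while Stop is true, and passes each bolt a struct of radius, color, branching and noise settings.
; StyleSelector picks random spherical or point-to-point arcs, with endpoints from vectors, actor locations or a random mesh vertex.
; A second self-repeating event randomizes core material brightness and light intensity.
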(event Custom|Arcing
  (bind _arc_struct (Variables|Default|GetArc%20Struct))
  (bind (_distance _boltcolor _isbranch _allowbranches _branchlimit _priorhitloc _priorhitnormal _playrate _customvectors _origin _dest _noisescale _noisespeed) (Utilities|Struct|BreakArcValues _arc_struct))
  ;[1 1 1] Create arc
  (if (Variables|Default|Getstop)
    (bind _returnvalue (Game|SpawnActorfromClass "/Game/Resources/Particles/Blueprints/BP_SpawnedArc.BP_SpawnedArc_C" (Transformation|GetActorTransform) "Undefined" self (Variables|Default|GetMovable) 0))
    (bind _output_get (|SetupArcStruct))
    (switch Utilities|FlowControl|Switch|SwitchonArcStyle (Variables|Default|GetStyle%20Selector)
      (:NewEnumerator0
        (Default|Spawn _returnvalue _output_get) ; Passing spawning values to arc
      )
      (:NewEnumerator1
        (|LocationLogic)
        (Default|Spawn _returnvalue (Utilities|Struct|MakeArcValues _distance _boltcolor _isbranch _allowbranches _branchlimit _priorhitloc _priorhitnormal _playrate true _origin _dest _noisescale _noisespeed)) ; Passing spawning values to arc
      )))
  ;[1 1 1] Spawn new arc
  (Utilities|FlowControl|Delay (Math|Random|RandomFloatinRange (Variables|Default|GetArc%20Min%20Delay) (Variables|Default|GetArc%20Max%20Delay)))
  (CallFunction|Arcing))

(event Custom|RandomCoreSize
  ;[1 1 1] Light setup for core (flickers size and brightness)
  (Rendering|Material|SetVectorParameterValue (Variables|Default|GetSphereMat) "Color" (* (Variables|Default|GetArcColor) (Math|Random|RandomFloatinRange 1.0 5.0)) :!class /Script/Engine.MaterialInstanceDynamic)
  (Rendering|Components|Light|SetIntensity (Variables|Default|GetPointLight) (Math|Random|RandomFloatinRange 3.2e+02 5e+03))
  (Utilities|FlowControl|Delay (Math|Random|RandomFloatinRange 0.05 0.09))
  (CallFunction|RandomCoreSize))

(event EventBeginPlay
  ;[1 1 1] Initialization
  (Utilities|Time|SetTimerbyFunctionName 0 "RandomCoreSize" 0.05)
  (Utilities|Time|SetTimerbyFunctionName 0 "Arcing" (Math|Random|RandomFloatinRange 0.05 0.025)))

(event Collision|EventActorBeginOverlap
  (params (OtherActor :type Actor%20Object%20Reference)))

(event EventTick
  (params (DeltaSeconds :type Float%20%28single-precision%29)))

(fn ConstructionScript
  (Components|Sphere|SetSphereRadius (Variables|Default|GetRadious%20Indicator) (Variables|Default|GetArc%20Radious) true)
  ;[1 1 1] Pass color to component
  (Rendering|Components|Light|SetLightColor (Variables|Default|GetPointLight) (Variables|Default|GetArcColor) true)
  (bind _returnvalue (Rendering|Material|CreateDynamicMaterialInstance (Variables|Default|GetStaticMesh) 0 0 "None" :!class /Script/Engine.PrimitiveComponent))
  (bind _output_get (Variables|Default|SetSphereMat _returnvalue))
  (Rendering|Material|SetVectorParameterValue _output_get "Color" (Variables|Default|GetArcColor) :!class /Script/Engine.MaterialInstanceDynamic)
  (Development|SetHiddeninGame (Variables|Default|GetStaticMesh) (not (Variables|Default|GetbCoreVisible)) false))