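; Energy shield actor that shows a fading ripple-style highlight at impact points, driven by either a RaycastHit event or physical component hits.
; Each hit creates a dynamic material instance, sets the impact position and radius, then animates opacity through a timeline; the component-hit path ends with a debug print.
; The construction script picks grey for impassable, blue with an overlap response for open, or red otherwise.
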(event OnComponentHit(StaticMesh)
  (params (HitComponent :type Primitive%20Component%20Object%20Reference) (OtherActor :type Actor%20Object%20Reference) (OtherComp :type Primitive%20Component%20Object%20Reference) (NormalImpulse :type Vector :default "0, 0, 0") (Hit :type Hit%20Result%20Structure%20%28by%20ref%29))
  (bind _staticmesh (Variables|Default|GetStaticMesh))
  (bind _returnvalue (Rendering|Material|CreateDynamicMaterialInstance _staticmesh 0 (Rendering|Material|GetMaterial _staticmesh 0) "None" :!class /Script/Engine.PrimitiveComponent))
  (Rendering|Material|SetVectorParameterValue _returnvalue "Pos" (Math|Conversions|ToLinearColor(Vector) (.impactpoint Hit)) :!class /Script/Engine.MaterialInstanceDynamic)
  (Rendering|Material|SetScalarParameterValue _returnvalue "Radius" (Variables|Default|GetHit%20Size) :!class /Script/Engine.MaterialInstanceDynamic)
  (bind _fade_time (Timeline|Timeline_0 PlayFromStart)
    (:Update
      (Rendering|Material|SetScalarParameterValue _returnvalue "Opacity" _fade_time :!class /Script/Engine.MaterialInstanceDynamic))
    (:Finished
      (Development|PrintString "Hello"))))

(event Custom|Raycast%20Hit
  (params (Other%20Comp :type Hit%20Result%20Structure))
  (bind _staticmesh (Variables|Default|GetStaticMesh))
  (bind _returnvalue (Rendering|Material|CreateDynamicMaterialInstance _staticmesh 0 (Rendering|Material|GetMaterial _staticmesh 0) "None" :!class /Script/Engine.PrimitiveComponent))
  (Rendering|Material|SetVectorParameterValue _returnvalue "Pos" (Math|Conversions|ToLinearColor(Vector) (.impactpoint Other%20Comp)) :!class /Script/Engine.MaterialInstanceDynamic)
  (Rendering|Material|SetScalarParameterValue _returnvalue "Radius" (Variables|Default|GetHit%20Size) :!class /Script/Engine.MaterialInstanceDynamic)
  (bind _fade_time (Timeline|Fade_Time PlayFromStart)
    (:Update
      (Rendering|Material|SetScalarParameterValue _returnvalue "Opacity" _fade_time :!class /Script/Engine.MaterialInstanceDynamic))))

(event EventBeginPlay)

(event Collision|EventActorBeginOverlap
  (params (OtherActor :type Actor%20Object%20Reference)))

(event EventTick
  (params (DeltaSeconds :type Float%20%28single-precision%29)))

(fn ConstructionScript
  (bind _staticmesh (Variables|Default|GetStaticMesh))
  (Collision|SetCollisionObjectType (Variables|Default|GetStaticMesh) "ECC_GameTraceChannel17")
  (if (Variables|Default|GetIs%20Impasable)
    (Rendering|Material|SetMaterial _staticmesh 0 "/Game/Resources/Particles/ParticleMaterials/M_Energy_Shield_V2_Grey.M_Energy_Shield_V2_Grey")
    (elif (Variables|Default|GetIs%20Open)
      (Rendering|Material|SetMaterial _staticmesh 0 "/Game/Resources/Particles/ParticleMaterials/M_Energy_Shield_V2_Blue.M_Energy_Shield_V2_Blue")
      (Collision|SetCollisionResponsetoChannel _staticmesh "ECC_GameTraceChannel1" "ECR_Overlap")
      (else
        (Rendering|Material|SetMaterial _staticmesh 0 "/Game/Resources/Particles/ParticleMaterials/M_Energy_Shield_V2_Red.M_Energy_Shield_V2_Red")))))