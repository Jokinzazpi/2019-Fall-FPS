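; Short-lived electric arc actor that, on Spawn, strikes a random traced surface point or spans two custom points given by its arc struct.
; It builds a spline mesh with a dynamic noise material, a point light and impact particles; a Countdown timeline animates bolt and light flicker, then destroys the actor.
; Hits can recursively spawn delayed branch arcs up to a limit, while non-branch arcs can keep their start attached to the moving owner.
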(event Custom|Spawn
  (params (ArcStruc :type Arc%20Values%20Structure))
  (bind _returnvalue (Transformation|GetActorLocation))
  (bind _custompos (Variables|Default|GetCustomPos))
  (|ArcStructExtraction ArcStruc)
  (|SetArcLifetime)
  (if (Variables|Default|GetCustomPos)
    _
    (else
      ;[1 1 1] Trace to find endpoint
      (bind _outhit (|FindArcEndpoint))
      (Variables|Default|SetTraceHit (.bBlockingHit (Collision|BreakHitResult _outhit)))
      (Variables|Default|SetHitLoc (.Location (Collision|BreakHitResult _outhit)))
      (Variables|Default|SetHitNormal (.ImpactNormal (Collision|BreakHitResult _outhit)))
      (Variables|Default|SetStartTangent (- (Transformation|GetActorLocation) (.TraceEnd (Collision|BreakHitResult _outhit))))
      (|HandleBranching
        (:else
          _))))
  (|CreateSpline)
  (|CreatePointlight)
  (|CreateParticles)
  ;[1 1 1] Use the trace results to build the endpoints for the spline
  (SplineMesh|SetStartandEnd (Variables|Default|GetSpline) (Math|Vector|SelectVector (Variables|Default|GetCustomLoc_D) (- (Math|Vector|SelectVector (Variables|Default|GetPriorHitLoc) _returnvalue (Variables|Default|GetbIs%20Branch)) (Transformation|GetActorLocation)) _custompos) (Math|Vector|SelectVector "0, 0,1.000000" (* (Math|Vector|Normalize (Math|Vector|SelectVector (Variables|Default|GetPriorHitNormal) (Variables|Default|GetStartTangent) (Variables|Default|GetbIs%20Branch))) (* (/ (Math|Vector|VectorLength (- (Variables|Default|GetHitLoc) (Transformation|GetActorLocation))) (Variables|Default|GetMax%20Distance)) -5e+02)) _custompos) (Math|Vector|SelectVector (Variables|Default|GetCustomLoc_O) (- (Variables|Default|GetHitLoc) _returnvalue) _custompos) (Math|Vector|SelectVector "0, 0,1.000000" (* (Variables|Default|GetHitNormal) (* (/ (Math|Vector|VectorLength (- (Variables|Default|GetHitLoc) (Transformation|GetActorLocation))) (Variables|Default|GetMax%20Distance)) -5e+02)) _custompos) true :!class /Script/Engine.SplineMeshComponent)
  ;;[1 1 1] Sets the direction the spline with 'ladder' up
  (Rendering|Material|SetVectorParameterValue (Variables|Default|GetArcMat) "BiasVector" (Math|Conversions|ToLinearColor(Vector) (* (Math|Vector|SelectVector "0, 0,1.000000" (+ (Math|Vector|Normalize (Math|Vector|SelectVector (Variables|Default|GetPriorHitNormal) (Variables|Default|GetStartTangent) (Variables|Default|GetbIs%20Branch))) (Variables|Default|GetHitNormal)) (Variables|Default|GetCustomPos)) 0.5)) :!class /Script/Engine.MaterialInstanceDynamic)
  (Variables|Default|SetBiasVector (* (Math|Vector|SelectVector "0, 0,1.000000" (+ (Math|Vector|Normalize (Math|Vector|SelectVector (Variables|Default|GetPriorHitNormal) (Variables|Default|GetStartTangent) (Variables|Default|GetbIs%20Branch))) (Variables|Default|GetHitNormal)) (Variables|Default|GetCustomPos)) 0.5))
  (if (Variables|Default|GetbIs%20Branch)
    _
    (elif (Variables|Default|GetbAllowUpdates)
      (CallFunction|SetMoving)))
  (|FinishArcs))

(event EventBeginPlay)

(event Collision|EventActorBeginOverlap
  (params (OtherActor :type Actor%20Object%20Reference)))

(event EventTick
  (params (DeltaSeconds :type Float%20%28single-precision%29)))

(fn ConstructionScript)

(event Custom|SpawnBranch
  (CallFunction|Spawn (stale _returnvalue) (Utilities|Struct|MakeArcValues (Variables|Default|GetMax%20Distance) (Variables|Default|GetNewColor) false false (- (Variables|Default|GetBranchCount) 1) (Variables|Default|GetHitLoc) (Variables|Default|GetHitNormal) (* (Components|Animation|GetPlayRate (Variables|Default|GetCountdown)) 1.15) false "0.000000,0.000000,0.000000" "0.000000,0.000000,0.000000" (Variables|Default|GetArc%20Noise) (Variables|Default|GetNoise%20Speed))))

(event Custom|StopMoving
  (bind (_endpos _endtangent) (|Inputs))
  (bind _spline (Variables|Default|GetSpline))
  (Utilities|FlowControl|Gate true) ; enters at Close
)

(event Custom|SetMoving
  (bind (_endpos _endtangent) (|Inputs))
  (bind _spline (Variables|Default|GetSpline))
  (Utilities|FlowControl|Gate true) ; enters at Open
)

(event EventTick
  (params (DeltaSeconds :type Float%20%28single-precision%29))
  (bind (_endpos _endtangent) (|Inputs))
  (bind _spline (Variables|Default|GetSpline))
  (if (Variables|Default|GetbAllowAnyTick)
    (if (Variables|Default|GetbTimeToDie)
      (Variables|Default|SetbAllowAnyTick false)
      (Utilities|FlowControl|Delay 0.5)
      (Actor|DestroyActor)
      (elif (not (Variables|Default|GetCustomPos))
        (Utilities|FlowControl|Gate true
          (:Exit
            (SplineMesh|SetStartandEnd _spline (- (Transformation|GetActorLocation (Components|GetOwner)) (Transformation|GetWorldLocation _spline)) "0, 0, 0" _endpos _endtangent true :!class /Script/Engine.SplineMeshComponent)))))))